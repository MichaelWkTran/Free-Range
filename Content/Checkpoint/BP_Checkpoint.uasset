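; Checkpoint actor for the chicken player that acts as the single active respawn point.
; On BeginPlay it destroys the checkpoint stored in ChikenRageGameGameMode and registers itself as the current one.
; RespawnPlayer teleports the PlayerChicken pawn to the checkpoint, zeroes its sphere's linear and angular physics velocity, and levels its rotation while keeping yaw.
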(event `self.ReceiveBeginPlay`
  (`self.K2_SetActorLocation` (`self.K2_GetActorLocation`))
  ;[1 1 1] Get Game Mode
  (bind _aschiken_rage_game_game_mode (cast `ChikenRageGameGameMode` (`GameplayStatics.GetGameMode`)))
  ;[1 1 1] Get Current Checkpoint
  (bind _asbp_checkpoint (cast `/Game/Checkpoint/BP_Checkpoint` (`ChikenRageGameGameMode.CurrentCheckpoint` _aschiken_rage_game_game_mode))
    (:`then`
      ;[1 1 1] Destroy Old Checkpoint
      (`self.DestroyCheckpoint` _asbp_checkpoint))
    (:`CastFailed`
      _))
  ;[1 1 1] Set to New Checkpoint
  (set `ChikenRageGameGameMode.CurrentCheckpoint` self _aschiken_rage_game_game_mode))

(fn `DestroyCheckpoint`
  (`self.K2_DestroyActor`))

(fn `RespawnPlayer`
  (bind _asplayer_chicken (cast `PlayerChicken` (`GameplayStatics.GetPlayerPawn` 0)))
  (`self.K2_SetActorLocation` _asplayer_chicken (`self.K2_GetActorLocation`) false true)
  (bind _spherecomponent (`PlayerChicken.SphereComponent` _asplayer_chicken))
  (`PrimitiveComponent.SetAllPhysicsLinearVelocity` _spherecomponent (0.0 0.0 0.0) false)
  (`PrimitiveComponent.SetPhysicsAngularVelocityInRadians` _spherecomponent (0.0 0.0 0.0) false "None")
  (bind (_returnvalue_roll _returnvalue_pitch _returnvalue_yaw) (`KismetMathLibrary.BreakRotator` (`self.K2_GetActorRotation` _asplayer_chicken)))
  (`self.K2_SetActorRotation` _asplayer_chicken (`KismetMathLibrary.MakeRotator` 0.0 0.0 _returnvalue_yaw) false))

(fn `UserConstructionScript`)