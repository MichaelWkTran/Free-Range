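; BP_CheckpointSpawner is a physics object that turns into a BP_Checkpoint once it comes to rest, unless it breaks first.
; A timeline serves as a settle timer, with a Delay on Update sampling velocity periodically and restarting it when speed exceeds a threshold.
; Hits above an impulse threshold destroy it while breakable.
; When the timeline finishes, it disables breaking, overlaps and physics, spawns the checkpoint at its transform and destroys itself.
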(event `self.ReceiveBeginPlay`
  (bind _staticmesh (`self.StaticMesh`))
  (`TimelineComponent.SetTimelineLength` (`self.Breakable Timeline`) (`self.Breakable Timeline Length`))
  ;[1 1 1] Wait until spawner  is in a stable position for a duration
  (`Timeline|Breakable Timeline` :!label _label
    (:`Update`
      (`KismetSystemLibrary.Delay` (/ (`self.Breakable Timeline Length`) (`self.Breakable Segement Factor`)))
      (if (> (`KismetMathLibrary.VSizeSquared` (`self.GetVelocity`)) (`KismetMathLibrary.Square` (`self.Breakable Reset Speed`)))
        (goto _label :!via `PlayFromStart`)))
    (:`Finished`
      ;[1 1 1] Create checkpoint when on a stable ground
      (`|ExecutionSequence`
        (:`then_0`
          (set `self.Is Breakable` false))
        (:`then_1`
          (set `PrimitiveComponent.bGenerateOverlapEvents` false _staticmesh))
        (:`then_2`
          (`PrimitiveComponent.SetSimulatePhysics` _staticmesh false)
          (`|SpawnActorFromClass` "/Game/Checkpoint/BP_Checkpoint.BP_Checkpoint_C" (`self.GetTransform`) "Undefined" "MultiplyWithRoot" null null)
          (`self.K2_DestroyActor`))))))

(event `self.StaticMesh.OnComponentHit`
  (params (HitComponent :type "PrimitiveComponent Object Reference") (OtherActor :type "Actor Object Reference") (OtherComp :type "PrimitiveComponent Object Reference") (NormalImpulse :type "Vector Structure") (Hit :type "HitResult Structure (by ref)"))
  ;[1 1 1] Destroy spawner when exceeding impulse
  (if (and (`self.Is Breakable`) (> (`KismetMathLibrary.VSizeSquared` NormalImpulse) (`KismetMathLibrary.Square` (`self.Break Impulse`))))
    (`self.K2_DestroyActor`)))

(fn `UserConstructionScript`)