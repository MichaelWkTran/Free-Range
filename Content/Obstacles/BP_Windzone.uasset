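; Wind zone obstacle that pushes physics-simulating objects overlapping its owning actor.
; Every tick it loops over the owner's overlapping actors and applies the Force vector, without acceleration change, to each one's primitive component if it simulates physics.
; A debug arrow showing the force direction from the owner's location is present but never runs.
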(event `self.ReceiveTick`
  (params (DeltaSeconds :type "Float (single-precision)"))
  (for _array_element (`Actor.GetOverlappingActors` (`self.GetOwner`) "/Script/Engine.Actor")
    (bind _returnvalue (`Actor.GetComponentByClass` _array_element "/Script/Engine.PrimitiveComponent"))
    (if (`SceneComponent.IsSimulatingPhysics` _returnvalue "None")
      (`PrimitiveComponent.AddForce` _returnvalue (`self.Force`) "None" false))))