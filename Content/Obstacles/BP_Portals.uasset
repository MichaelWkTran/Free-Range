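; BP_Portals is an obstacle holding two linked portals that teleport the PlayerChicken between each other.
; Overlapping an active portal disables the other and moves the chicken to that other portal's world location without sweeping.
; Leaving a portal's overlap re-arms it, so the active flags prevent an immediate bounce back on arrival.
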(event `self.Portal A.OnComponentBeginOverlap`
  (params (OverlappedComponent :type "PrimitiveComponent Object Reference") (OtherActor :type "Actor Object Reference") (OtherComp :type "PrimitiveComponent Object Reference") (OtherBodyIndex :type Integer) (bFromSweep :type Boolean) (SweepResult :type "HitResult Structure (by ref)"))
  (bind _asplayer_chicken (cast `PlayerChicken` OtherActor))
  (if (`self.Portal A Active`)
    (set `self.Portal B Active` false)
    (`self.K2_SetActorLocation` _asplayer_chicken (`SceneComponent.K2_GetComponentLocation` (`self.Portal B`)) false true)))

(event `self.Portal B.OnComponentBeginOverlap`
  (params (OverlappedComponent :type "PrimitiveComponent Object Reference") (OtherActor :type "Actor Object Reference") (OtherComp :type "PrimitiveComponent Object Reference") (OtherBodyIndex :type Integer) (bFromSweep :type Boolean) (SweepResult :type "HitResult Structure (by ref)"))
  (bind _asplayer_chicken (cast `PlayerChicken` OtherActor))
  (if (`self.Portal B Active`)
    (set `self.Portal A Active` false)
    (`self.K2_SetActorLocation` _asplayer_chicken (`SceneComponent.K2_GetComponentLocation` (`self.Portal A`)) false true)))

(event `self.Portal A.OnComponentEndOverlap`
  (params (OverlappedComponent :type "PrimitiveComponent Object Reference") (OtherActor :type "Actor Object Reference") (OtherComp :type "PrimitiveComponent Object Reference") (OtherBodyIndex :type Integer))
  (cast `PlayerChicken` OtherActor)
  (set `self.Portal A Active` true))

(event `self.Portal B.OnComponentEndOverlap`
  (params (OverlappedComponent :type "PrimitiveComponent Object Reference") (OtherActor :type "Actor Object Reference") (OtherComp :type "PrimitiveComponent Object Reference") (OtherBodyIndex :type Integer))
  (cast `PlayerChicken` OtherActor)
  (set `self.Portal B Active` true))

(fn `UserConstructionScript`)