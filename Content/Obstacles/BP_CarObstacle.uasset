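; A physics-driven car obstacle that follows a spline and explodes after an optional lifetime, when stuck, or on certain PlayerChicken hits.
; Each tick it yaws the front wheel components toward a velocity-scaled look-ahead spline point and rechecks low speed after a delay.
; Hits explode it unless body velocity opposes the impulse.
; Explosion adds effects, frees body and wheels as physics debris, radially pushes nearby bodies, draws a debug sphere, then destroys the actor.
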(event `self.ReceiveBeginPlay`
  (bind _lifetime (`self.Lifetime`))
  (if (> _lifetime 0.0)
    (`KismetSystemLibrary.Delay` _lifetime)
    (`self.Explode`)))

(event `self.ReceiveTick`
  (params (DeltaSeconds :type "Float (single-precision)"))
  (bind _spline (`self.Spline`))
  (bind (_returnvalue_x _returnvalue_y _returnvalue_z) (`KismetMathLibrary.BreakVector` (`KismetMathLibrary.Quat_Euler` (`KismetMathLibrary.Quat_FindBetweenVectors` (`KismetMathLibrary.Vector_Normal2D` (- (`SplineComponent.GetLocationAtDistanceAlongSpline` (`self.Spline`) (`KismetMathLibrary.FWrap` (+ (`KismetMathLibrary.VSizeXY` (* (`self.GetVelocity`) (`self.Look Forwad Scale`))) (`SplineComponent.GetDistanceAlongSplineAtSplineInputKey` _spline (`SplineComponent.FindInputKeyClosestToWorldLocation` _spline (`self.K2_GetActorLocation`)))) 0.0 (`SplineComponent.GetSplineLength` _spline)) "World") (`self.K2_GetActorLocation`))) (`KismetMathLibrary.Vector_Normal2D` (`self.GetActorForwardVector`))))))
  (if (not (`self.Has Exploded`))
    (`|ExecutionSequence`
      (:`then_0`
        (`/Engine/EditorBlueprintResources/StandardMacros.IsValid` (`self.Spline`)
          (:`Is Valid`
            (for _array_element (`|MakeArray` (`self.FL`) (`self.FR`))
              (`SceneComponent.K2_SetRelativeRotation` _array_element (`KismetMathLibrary.MakeRotator` 0.0 0.0 (`KismetMathLibrary.MapRangeClamped` (* _returnvalue_z -1.0) -360.0 360.0 -45.0 45.0)) false false)))))
      (:`then_1`
        (bind _returnvalue (`PrimitiveComponent.GetPhysicsLinearVelocity` (`self.Body`) "None"))
        (if (< (`KismetMathLibrary.VSizeXYSquared` _returnvalue) (`self.Explode Speed`))
          (`KismetSystemLibrary.Delay` (`self.Explode Time`))
          (bind _returnvalue_2 (`PrimitiveComponent.GetPhysicsLinearVelocity` (`self.Body`) "None"))
          (if (< (`KismetMathLibrary.VSizeXYSquared` _returnvalue_2) (`self.Explode Speed`))
            (`self.Explode`)))))))

(event `self.Body.OnComponentHit`
  (params (HitComponent :type "PrimitiveComponent Object Reference") (OtherActor :type "Actor Object Reference") (OtherComp :type "PrimitiveComponent Object Reference") (NormalImpulse :type "Vector Structure") (Hit :type "HitResult Structure (by ref)"))
  (if (not (`self.Has Exploded`))
    (cast `PlayerChicken` OtherActor)
    (bind _returnvalue (`PrimitiveComponent.GetPhysicsLinearVelocity` (`self.Body`) "None"))
    (if (not (< (`KismetMathLibrary.Dot_VectorVector` _returnvalue NormalImpulse) 0.0))
      (`self.Explode`))))

(event `Explode`
  (bind _returnvalue (`self.K2_GetActorLocation`))
  (bind _explosion_radius (`self.Explosion Radius`))
  (`|ExecutionSequence`
    (:`then_0`
      (set `self.Has Exploded` true)
      (bind _returnvalue_2 (`AddComponent|NODE_AddParticleSystemComponent-0`))
      (`SceneComponent.SetWorldScale3D` _returnvalue_2 (10.0 10.0 10.0))
      (`AddComponent|NODE_AddAudioComponent-0`)
      (for _array_element (`|MakeArray` (`self.BR`) (`self.FR`) (`self.FL`) (`self.BL`))
        (`ActorComponent.SetComponentTickEnabled` _array_element false)))
    (:`then_1`
      (for _array_element_2 (`|MakeArray` (`self.Body`) (`self.WheelFR`) (`self.WheelBR`) (`self.WheelBL`) (`self.WheelFL`))
        (`|ExecutionSequence`
          (:`then_0`
            (set `self.Part World Transform` (`SceneComponent.K2_GetComponentToWorld` _array_element_2))
            (`SceneComponent.SetAbsolute` _array_element_2 true true true)
            (`SceneComponent.K2_SetWorldTransform` _array_element_2 (`self.Part World Transform`) false false))
          (:`then_1`
            (`PrimitiveComponent.SetSimulatePhysics` _array_element_2 true)
            (`PrimitiveComponent.SetCollisionEnabled` _array_element_2 "PhysicsOnly")
            (`PrimitiveComponent.SetCollisionObjectType` _array_element_2 "ECC_PhysicsBody")
            (`PrimitiveComponent.SetMassScale` _array_element_2 "None" 0.01)))))
    (:`then_2`
      (bind _outcomponents (`KismetSystemLibrary.SphereOverlapComponents` _returnvalue _explosion_radius (`|MakeArray` "ObjectTypeQuery2" "ObjectTypeQuery3" "ObjectTypeQuery4" "ObjectTypeQuery5" "ObjectTypeQuery6" :!type "EObjectTypeQuery Enum") "/Script/Engine.PrimitiveComponent"))
      (`KismetSystemLibrary.DrawDebugSphere` _returnvalue _explosion_radius 12 (struct :`G` 1.0 :`A` 1.0) 5.0)
      (for _array_element_3 _outcomponents
        (if (`SceneComponent.IsSimulatingPhysics` _array_element_3 "None")
          (`PrimitiveComponent.AddRadialImpulse` _array_element_3 (`self.K2_GetActorLocation`) (`self.Explosion Radius`) (`self.Explosion Strength`) "RIF_Linear" false))))
    (:`then_3`
      (`KismetSystemLibrary.Delay` (`self.Destroy Time`))
      (`self.K2_DestroyActor`))))

(fn `UserConstructionScript`)