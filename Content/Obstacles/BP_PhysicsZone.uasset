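; BP_PhysicsZone is a physics drag zone that slows fast-moving simulated objects overlapping its owner.
; Every Tick it loops over the owner's overlapping actors, checking whether each one's PrimitiveComponent simulates physics and moves faster than MinSpeed.
; Those components receive a force opposing the actor's velocity, scaled by excess speed and ForceStrength, with AccelChange controlling whether it is applied as acceleration.
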(event `self.ReceiveTick`
  (params (DeltaSeconds :type "Float (single-precision)"))
  (for _array_element (`Actor.GetOverlappingActors` (`self.GetOwner`) "/Script/Engine.Actor")
    (bind _returnvalue (`Actor.GetComponentByClass` _array_element "/Script/Engine.PrimitiveComponent"))
    (if (`SceneComponent.IsSimulatingPhysics` _returnvalue "None")
      (bind _returnvalue_2 (`KismetMathLibrary.VSize` (`SceneComponent.GetComponentVelocity` _returnvalue)))
      (if (> _returnvalue_2 (`self.Min Speed`))
        (`PrimitiveComponent.AddForce` _returnvalue (* (* (- _returnvalue_2 (`self.Min Speed`)) (`self.Force Strength`)) (`KismetMathLibrary.NegateVector` (`KismetMathLibrary.Normal` (`Actor.GetVelocity` _array_element)))) "None" (`self.Accel Change`))))))