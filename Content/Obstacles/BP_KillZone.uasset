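; Kill zone Blueprint that destroys actors overlapping its owner.
; On BeginPlay it binds a handler to the owner's ActorBeginOverlap event.
; The handler destroys any overlapping actor when the ActorsToDestroy class list is empty, otherwise only actors matching one of the listed classes.
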(event `self.ReceiveBeginPlay`
  (add `Actor.OnActorBeginOverlap` (`self.GetOwner`) (delegate `OnActorBeginOverlap`)))

(event `OnActorBeginOverlap`
  (params (OverlappedActor :type "Actor Object Reference") (OtherActor :type "Actor Object Reference"))
  (bind _actors_to_destroy (`self.Actors To Destroy`))
  (if (<= (`KismetArrayLibrary.Array_Length` _actors_to_destroy) 0)
    (`Actor.K2_DestroyActor` OtherActor)
    (else
      (for _array_element _actors_to_destroy
        (if (`GameplayStatics.ObjectIsA` OtherActor _array_element)
          (`Actor.K2_DestroyActor` OtherActor)
          (break))))))