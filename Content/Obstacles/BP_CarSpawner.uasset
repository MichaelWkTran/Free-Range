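; BP_CarSpawner is an obstacle actor that endlessly spawns vehicles at its own transform.
; From BeginPlay, a self-restarting Delay loop waits a random time between Min and Max before each spawn.
; Each vehicle is picked at random from VehiclesToSpawn and launched along the spawner's forward vector with a velocity-change impulse on its Body.
; It also receives the SplineComponent found on the referenced Spline actor.
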(event `self.ReceiveBeginPlay`
  (`KismetSystemLibrary.Delay` (`KismetMathLibrary.RandomFloatInRange` (`self.Min`) (`self.Max`)) :!label _label)
  (`|ExecutionSequence`
    (:`then_0`
      (goto _label))
    (:`then_1`
      (bind _returnvalue (`|SpawnActorFromClass` (`KismetArrayLibrary.Array_Random` (`self.Vehicles To Spawn`)) (`self.GetTransform`) "Undefined" "MultiplyWithRoot" null null))
      (`PrimitiveComponent.AddImpulse` (`/Game/Obstacles/BP_CarObstacle.Body` _returnvalue) (* (`self.GetActorForwardVector`) (`self.Spawn Velocity`)) "None" true)
      (set `/Game/Obstacles/BP_CarObstacle.Spline` (`self.GetComponentByClass` (`self.Spline`) "/Script/Engine.SplineComponent") _returnvalue))))

(fn `UserConstructionScript`)