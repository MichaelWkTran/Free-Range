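; Spline-shaped treadmill obstacle that pushes actors touching it along the direction of its spline.
; The construction script builds a spline mesh between each pair of spline points, with a configurable width or height scale.
; On actor hit, a normal-Z check filters contacts by facing, then the spline direction nearest the other actor is scaled by TreadmillSpeed.
; UseForce selects between a physics force and a non-swept world offset applied per hit.
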(event `self.ReceiveBeginPlay`
  (add `self.OnActorHit` (delegate `OnActorHit_Event`)))

(event `OnActorHit_Event` :!signature `self.OnActorHit`
  (params (SelfActor :type "Actor Object Reference") (OtherActor :type "Actor Object Reference") (NormalImpulse :type "Vector Structure") (Hit :type "HitResult Structure (by ref)"))
  (bind _returnvalue (* (`SplineComponent.FindDirectionClosestToWorldLocation` (`self.Spline`) (`self.K2_GetActorLocation` OtherActor) "World") (`self.Treadmill Speed`)))
  (if (< (.z (`.Normal` (`GameplayStatics.BreakHitResult` Hit))) -0.5)
    (if (`self.Use Force`)
      (`PrimitiveComponent.AddForce` Hit_HitComponent _returnvalue "None" false)
      (else
        (`self.K2_AddActorWorldOffset` OtherActor _returnvalue false false)))))

(fn `UserConstructionScript`
  (bind _spline (`self.Spline`))
  (bind _spline_end_scale (`self.Spline End Scale`))
  (for _index (range (+ (- (`SplineComponent.GetNumberOfSplinePoints` (`self.Spline`)) 2) 1))
    (bind _returnvalue (`AddComponent|NODE_AddSplineMeshComponent-0`))
    (bind _returnvalue_2 (+ _index 1))
    (`SplineMeshComponent.SetStartAndEnd` _returnvalue (`SplineComponent.GetLocationAtSplinePoint` _spline _index "Local") (`SplineComponent.GetTangentAtSplinePoint` _spline _index "Local") (`SplineComponent.GetLocationAtSplinePoint` _spline _returnvalue_2 "Local") (`SplineComponent.GetTangentAtSplinePoint` _spline _returnvalue_2 "Local") true)
    (`SplineMeshComponent.SetEndScale` _returnvalue (`KismetMathLibrary.MakeVector2D` _spline_end_scale 1.0) true)
    (`SplineMeshComponent.SetStartScale` _returnvalue (`KismetMathLibrary.MakeVector2D` _spline_end_scale 1.0) true)))