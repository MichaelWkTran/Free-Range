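; Moving platform loop obstacle that carries an array of platform actors along a spline at a set speed, wrapping at the ends.
; The construction script snaps each platform to its closest spline point, and Tick derives each one's next distance from its current location.
; Overlapping physics-simulating actors receive the same offset before each platform teleports.
; A ReverseSpline helper flips direction by rebuilding points with reversed input keys.
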(event `self.ReceiveTick`
  (params (DeltaSeconds :type "Float (single-precision)"))
  (bind _spline (`self.Spline`))
  (for _array_element (`self.Platforms`)
    (`/Engine/EditorBlueprintResources/StandardMacros.IsValid` _array_element
      (:`Is Valid`
        (for _array_element_2 (`self.GetOverlappingActors` _array_element null)
          (bind _returnvalue (`self.GetComponentByClass` _array_element_2 "/Script/Engine.PrimitiveComponent"))
          (`/Engine/EditorBlueprintResources/StandardMacros.IsValid` _returnvalue
            (:`Is Valid`
              (if (`SceneComponent.IsSimulatingPhysics` _returnvalue "None")
                (bind _returnvalue_2 (`SplineComponent.GetLocationAtDistanceAlongSpline` (`self.Spline`) (`KismetMathLibrary.FWrap` (+ (* DeltaSeconds (`self.Speed`)) (`SplineComponent.GetDistanceAlongSplineAtSplineInputKey` _spline (`SplineComponent.FindInputKeyClosestToWorldLocation` _spline (`self.K2_GetActorLocation` _array_element)))) 0.0 (`SplineComponent.GetSplineLength` _spline)) "World"))
                (`self.K2_AddActorWorldOffset` _array_element_2 (- _returnvalue_2 (`self.K2_GetActorLocation` _array_element)) false false)))))
        (`self.K2_SetActorLocation` _array_element _returnvalue_2 false true)))))

(fn `Reverse Spline`
  (locals (`Spline Points` :type "Array of SplinePoint Structure"))
  (bind _spline (`self.Spline`))
  (for _index (range (`SplineComponent.GetNumberOfSplinePoints` (`self.Spline`)))
    (`KismetArrayLibrary.Array_Add` (`local.Spline Points`) (make `SplinePoint` (`KismetMathLibrary.Conv_IntToDouble` (- (- (`SplineComponent.GetNumberOfSplinePoints` (`self.Spline`)) 1) _index)) (`SplineComponent.GetLocationAtSplinePoint` _spline _index "Local") (`SplineComponent.GetArriveTangentAtSplinePoint` _spline _index "Local") (`SplineComponent.GetLeaveTangentAtSplinePoint` _spline _index "Local") (`SplineComponent.GetRotationAtSplinePoint` _spline _index "Local") (`SplineComponent.GetScaleAtSplinePoint` _spline _index) (`SplineComponent.GetSplinePointType` _spline _index))))
  (`SplineComponent.ClearSplinePoints` (`self.Spline`) false)
  (`SplineComponent.AddPoints` (`self.Spline`) (`local.Spline Points`) true))

(fn `Snap Platforms`
  (for _array_element (`self.Platforms`)
    (`/Engine/EditorBlueprintResources/StandardMacros.IsValid` _array_element
      (:`Is Valid`
        (`self.K2_SetActorLocation` _array_element (`SplineComponent.FindLocationClosestToWorldLocation` (`self.Spline`) (`self.K2_GetActorLocation` _array_element) "World") false true)))))

(fn `UserConstructionScript`
  (`self.Snap Platforms`))